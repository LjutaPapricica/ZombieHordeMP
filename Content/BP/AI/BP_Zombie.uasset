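; Zombie enemy with networked damage, per-bone dismemberment and a physics-driven crawl toward its attacker.
; Server damage is multicast to lower HP, play hit effects and wear down bone durability, with upper-spine and pelvis hits counted as spine_01.
; A broken bone ragdolls the body, then after a delay Tick pulls hands and head toward the damage causer, moving the capsule along.
; Zero HP triggers a final ragdoll impulse and timed removal.
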(event `self.ReceiveBeginPlay`
  (`PhysicalAnimationComponent.SetSkeletalMeshComponent` (`self.PhysicalAnimation`) (`self.Mesh`)))

(event `server_OnTakeDamage`
  (params (Damage :type "Float (double-precision)") (DamageCauser :type "Actor Object Reference") (HitBoneName :type Name))
  (`self.multicast_OnTakeDamage` Damage DamageCauser HitBoneName))

(event `multicast_OnTakeDamage`
  (params (Damage :type "Float (double-precision)") (DamageCauser :type "Actor Object Reference") (HitBoneName :type Name))
  (set `self.DamageCauser` DamageCauser)
  (set `self.HitBoneName` HitBoneName)
  (bind _hp (`self.TakeDamage` Damage))
  (if (<= _hp 0.0)
    (`self.Dead`)))

(event `Dead`
  (bind _mesh (`self.Mesh`))
  (`PrimitiveComponent.SetCollisionEnabled` (`self.CapsuleComponent`) "NoCollision")
  (`PrimitiveComponent.SetSimulatePhysics` _mesh true)
  (`PrimitiveComponent.SetCollisionEnabled` _mesh "PhysicsOnly")
  (`PrimitiveComponent.AddImpulseAtLocation` (`self.Mesh`) (* (`KismetMathLibrary.GetForwardVector` (`self.K2_GetActorRotation` (`self.DamageCauser`))) (`KismetMathLibrary.RandomFloatInRange` 6000.0 12000.0)) (0.0 0.0 0.0) (`self.HitBoneName`))
  (set `self.NewVar_0` false)
  (`self.SetLifeSpan` 30.0))

(event `NearDeath`
  (`PrimitiveComponent.SetSimulatePhysics` (`self.Mesh`) true)
  (`PrimitiveComponent.SetCollisionEnabled` (`self.CapsuleComponent`) "NoCollision")
  (`PrimitiveComponent.AddImpulseAtLocation` (`self.Mesh`) (* (`KismetMathLibrary.GetForwardVector` (`self.K2_GetActorRotation` (`self.DamageCauser`))) (`KismetMathLibrary.RandomFloatInRange` 3000.0 6000.0)) (0.0 0.0 0.0) (`self.HitBoneName`))
  (`KismetSystemLibrary.Delay` (`KismetMathLibrary.RandomFloatInRange` 2.0 3.0))
  (set `self.NewVar_0` true))

(event `self.ReceiveTick`
  (params (DeltaSeconds :type "Float (single-precision)"))
  (bind _mesh (`self.Mesh`))
  (bind _returnvalue (+ (* (`KismetMathLibrary.ClampVectorSize` (`KismetMathLibrary.GetForwardVector` (`KismetMathLibrary.FindLookAtRotation` (`SceneComponent.K2_GetComponentLocation` (`self.CapsuleComponent`)) (`self.K2_GetActorLocation` (`self.DamageCauser`)))) 0.0 1.0) (`self.ForwardForce`)) (`KismetMathLibrary.MakeVector` 0.0 0.0 (`self.ZForce`))))
  (if (and (`self.NewVar_0`) (> (`self.HP`) 0.0))
    (`PrimitiveComponent.AddForce` _mesh _returnvalue "hand_r" true)
    (`PrimitiveComponent.AddForce` _mesh _returnvalue "hand_l" true)
    (`PrimitiveComponent.AddForce` _mesh _returnvalue "head" true)
    (`SceneComponent.K2_SetWorldLocation` (`self.CapsuleComponent`) (`SceneComponent.GetSocketLocation` _mesh "head") false false)))

(fn `Dismemberment`
  (params (Damage :type "Float (double-precision)"))
  (bind (_value _returnvalue) (`BlueprintMapLibrary.Map_Find` (`self.BoneDurable`) (`self.HitBoneName`)))
  (if _returnvalue
    (`BlueprintMapLibrary.Map_Add` (`self.BoneDurable`) (`self.HitBoneName`) (- _value Damage))
    (if (<= (`BlueprintMapLibrary.Map_Find` (`self.BoneDurable`) (`self.HitBoneName`)) 0.0)
      (`SkeletalMeshComponent.BreakConstraint` (`self.Mesh`) (* (`KismetMathLibrary.GetForwardVector` (`self.K2_GetActorRotation` (`self.DamageCauser`))) (`KismetMathLibrary.RandomFloatInRange` 3000.0 5000.0)) (0.0 0.0 0.0) (`self.HitBoneName`))
      (switch `name` (`self.HitBoneName`)
        (:`spine_01`
          (set `self.ZForce` 1500.0)
          (set `self.ForwardForce` 3000.0))
        (:`thigh_r`
          (set `self.ZForce` 1800.0 :!label _label)
          (set `self.ForwardForce` 4200.0))
        (:`thigh_l`
          (goto _label))
        (:`calf_r`
          (goto _label))
        (:`calf_l`
          (goto _label))
        (:`foot_r`
          (goto _label))
        (:`foot_l`
          (goto _label)))
      (`self.NearDeath`))))

(fn `NormalizeBoneName`
  (switch `name` (`self.HitBoneName`)
    (:`spine_02`
      _)
    (:`spine_03`
      _)
    (:`pelvis`
      _))
  (set `self.HitBoneName` "spine_01"))

(fn `TakeDamage`
  (params (Damage :type "Float (double-precision)"))
  (returns (HP :type "Float (double-precision)"))
  (bind _output_get (set `self.HP` (- (`self.HP`) Damage)))
  (`GameplayStatics.SpawnEmitterAttached` "/Game/Effects/ParticleSystems/Gameplay/Player/P_body_bullet_impact.P_body_bullet_impact" (`self.Mesh`) (`self.HitBoneName`) (0.0 0.0 0.0) (struct) (1.5 1.5 1.5))
  (`GameplayStatics.SpawnSoundAtLocation` "/Game/Sounds/FoleyFlesh/Stereo/Dismemberment_Cue.Dismemberment_Cue" (`self.K2_GetActorLocation`) (struct) 0.05 1.0 0.0 null null)
  (`self.NormalizeBoneName`)
  (`self.Dismemberment` Damage)
  (return _output_get))

(fn `UserConstructionScript`)