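; BP_ZombieCon is a zombie AI controller with logic for chasing the nearest player.
; SearchNearestPlayer scans the Players array by horizontal distance to the controlled pawn and stores the closest as ChaseToPlayer, without resetting the stored minimum distance.
; MoveToPlayer sends the pawn toward that target with SimpleMoveToActor when it is valid.
; BeginPlay is empty, and the looping timer setup for both events is disconnected, so nothing here triggers them.
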(event `self.ReceiveBeginPlay`)

(event `MoveToPlayer`
  ;[1 1 1] Comment
  (bind _chasetoplayer (`self.ChaseToPlayer`)
    (:`then`
      (`AIBlueprintHelperLibrary.SimpleMoveToActor` self _chasetoplayer))
    (:`else`)))

(event `SearchNearestPlayer`
  ;[1 1 1] Comment
  (for (_array_element _array_index) (`self.Players`)
    (bind _returnvalue (`self.GetHorizontalDistanceTo` (`self.K2_GetPawn`) _array_element))
    (if (> (`self.MinDistanceToPlayer`) _returnvalue)
      (set `self.MinDistanceToPlayer` _returnvalue)
      (set `self.NearestPlayerIndex` _array_index)))
  (set `self.ChaseToPlayer` (`|GetArrayItem` (`self.Players`) (`self.NearestPlayerIndex`))))

(fn `UserConstructionScript`)